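; AI performance profiling player character Blueprint that relocates itself on a timer.
; Tick accumulates elapsed Runtime and, once it passes PlayTime, sets the actor to a fixed location every frame.
; After PlayTimeRetrun it also moves the actor to a second fixed location on the opposite side of the X axis.
; A DestroyActor call is present but unconnected, and the construction script is empty.
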(event EventTick
  (params (DeltaSeconds :type Float%20%28single-precision%29))
  (bind _output_get (Variables|Default|SetRuntime (+ DeltaSeconds (Variables|Default|GetRuntime))))
  (if (>= _output_get (Variables|Default|GetPlayTime))
    (Transformation|SetActorLocation "2000.000000,0.000000,90.000000" false false)
    (if (>= (Variables|Default|GetRuntime) (Variables|Default|GetPlayTime_Retrun))
      (Transformation|SetActorLocation "-2000.000000,0.000000,90.000000" false false))))

(fn ConstructionScript)