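; Sword weapon actor that plays a dissolve effect with a material and Niagara particles.
; BeginPlay creates a dynamic dissolve material on the skeletal mesh and sets its Amount to 1.
; Dissolve events spawn attached Niagara, pass the incoming amount to material and particles, then hide the mesh and deactivate the particles.
; The per-update material write uses parameter name None instead of Amount, unlike the Niagara write.
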(event EventBeginPlay
  (bind _returnvalue (Rendering|Material|CreateDynamicMaterialInstance (Variables|Default|GetSkeletalMesh) 0 (Variables|Default|GetDissolveMaterial) "None" :!class /Script/Engine.PrimitiveComponent))
  (bind _output_get (Variables|Default|SetDissolveMID _returnvalue))
  (Rendering|Material|SetScalarParameterValue _output_get "Amount" 1.0 :!class /Script/Engine.MaterialInstanceDynamic))

(event EventWeaponDissolveStarted
  (bind _returnvalue (Niagara|SpawnSystemAttached (Variables|Default|GetDissolveNiagara) (Variables|Default|GetSkeletalMesh) "None" "0, 0, 0" "0, 0, 0" "KeepRelativeOffset" true))
  (Utilities|IsValid _returnvalue
    (:Is%20Valid
      (Variables|Default|SetDissolveNiagaraComponent _returnvalue))))

(event EventWeaponDissolveAmount
  (params (InAmount :type Float%20%28single-precision%29))
  (bind _dissolvemid (Variables|Default|GetDissolveMID))
  (bind _dissolveniagaracomponent (Variables|Default|GetDissolveNiagaraComponent))
  (Utilities|FlowControl|Sequence
    (:then_0
      (Utilities|IsValid _dissolvemid
        (:Is%20Valid
          (Rendering|Material|SetScalarParameterValue _dissolvemid "None" InAmount :!class /Script/Engine.MaterialInstanceDynamic))))
    (:then_1
      (Utilities|IsValid _dissolveniagaracomponent
        (:Is%20Valid
          (Niagara|SetNiagaraVariable(Float) _dissolveniagaracomponent "Amount" InAmount))))))

(event EventWeaponDissolveFinished
  (Rendering|SetVisibility (Variables|Default|GetSkeletalMesh) false false)
  (Components|Activation|Deactivate (Variables|Default|GetDissolveNiagaraComponent)))

(fn ConstructionScript)